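; BP_ProximityExplosion is a one-shot explosive actor that detonates when the player enters its trigger radius.
; BeginPlay sizes TriggerSphere from TriggerRadius, and its overlap event filters for player character 0, passes a DoOnce gate, then casts to BP_FirstPersonCharacterShooter.
; Detonation spawns the explosion effect, fires the RFExplosion impulse, plays a distance-based camera shake and attenuated sound, then destroys the actor.
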(event `self.ReceiveBeginPlay`
  (`SphereComponent.SetSphereRadius` (`self.TriggerSphere`) (`self.TriggerRadius`) true))

(event `self.TriggerSphere.OnComponentBeginOverlap`
  (params (OverlappedComponent :type "PrimitiveComponent Object Reference") (OtherActor :type "Actor Object Reference") (OtherComp :type "PrimitiveComponent Object Reference") (OtherBodyIndex :type Integer) (bFromSweep :type Boolean) (SweepResult :type "HitResult Structure (by ref)"))
  (if (== OtherActor (`GameplayStatics.GetPlayerCharacter` 0))
    (`/Engine/EditorBlueprintResources/StandardMacros.DoOnce` false
      (:`Completed`
        (cast `/Game/FirstPerson/Blueprints/BP_FirstPersonCharacterShooter` OtherActor)
        (`NiagaraFunctionLibrary.SpawnSystemAtLocation` "/Game/NiagaraExamples/FX_Explosions/NS_Explosion.NS_Explosion" (`self.K2_GetActorLocation`) (`self.K2_GetActorRotation`))
        (`RadialForceComponent.FireImpulse` (`self.RF_Explosion`))
        (`GameplayStatics.PlayWorldCameraShake` "/Game/CS_Explosion.CS_Explosion_C" (`self.K2_GetActorLocation`) 300.0 5000.0)
        (`GameplayStatics.PlaySoundAtLocation` "/Game/Sounds/SC_Explosion.SC_Explosion" (`self.K2_GetActorLocation`) (struct) 1.0 1.0 0.0 "/Game/Sounds/ACC_ExplosionHangar.ACC_ExplosionHangar" null null null)
        (`self.K2_DestroyActor`)))))

(fn `UserConstructionScript`)