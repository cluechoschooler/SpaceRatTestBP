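; BP_AlarmDirector is an actor that plays an endlessly looping sequence of alarm sounds.
; On BeginPlay it starts the first sound in the AlarmPattern array, then advances PatternIndex with modulo wrap-around.
; The audio component's OnAudioFinished event triggers the next sound, chaining the pattern.
; Debug prints trace each step.
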(event `self.ReceiveBeginPlay`
  (`KismetSystemLibrary.PrintString` "Begin")
  (`self.PlayNextAlarm`))

(event `PlayNextAlarm`
  (bind _output (`|GetArrayItem` (`self.AlarmPattern`) (`self.PatternIndex`)))
  (`KismetSystemLibrary.PrintString` "next")
  (`AudioComponent.Stop` (`self.AC_Alarm`))
  (`KismetSystemLibrary.PrintString` (`KismetSystemLibrary.GetDisplayName` _output))
  (`AudioComponent.SetSound` (`self.AC_Alarm`) _output)
  (`AudioComponent.Play` (`self.AC_Alarm`) 0.0)
  (`KismetSystemLibrary.PrintString` (`KismetStringLibrary.Conv_IntToString` (`self.PatternIndex`)))
  (set `self.PatternIndex` (mod (+ (`self.PatternIndex`) 1) (`KismetArrayLibrary.Array_Length` (`self.AlarmPattern`)))))

(event `self.AC_Alarm.OnAudioFinished`
  (`self.PlayNextAlarm`)
  (`KismetSystemLibrary.PrintString` "FINISHED"))

(fn `UserConstructionScript`)