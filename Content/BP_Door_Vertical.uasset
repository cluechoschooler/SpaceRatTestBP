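; Vertical sliding door that opens while the player character stands inside its trigger box and closes when they leave.
; BeginPlay stores the panel's closed location and derives the open one by adding a Z offset of OpenDistance.
; Overlap begin and end toggle a WantsOpen flag and play the same door sound.
; Tick continuously interpolates the panel toward the selected location with VInterpTo at OpenSpeed, without a Timeline.
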(event `self.ReceiveBeginPlay`
  (`|ExecutionSequence`
    (:`then_0`
      (bind _output_get (set `self.ClosedLoc` (`SceneComponent.RelativeLocation` (`self.SM_DoorPanel`))))
      (set `self.OpenLoc` (+ _output_get (`KismetMathLibrary.MakeVector` 0.0 0.0 (`self.OpenDistance`)))))))

(event `self.OpenDoor_Box_Small.OnComponentBeginOverlap`
  (params (OverlappedComponent :type "PrimitiveComponent Object Reference") (OtherActor :type "Actor Object Reference") (OtherComp :type "PrimitiveComponent Object Reference") (OtherBodyIndex :type Integer) (bFromSweep :type Boolean) (SweepResult :type "HitResult Structure (by ref)"))
  (if (== OtherActor (`GameplayStatics.GetPlayerCharacter` 0))
    (set `self.WantsOpen ` true)
    (`GameplayStatics.PlaySoundAtLocation` "/Game/Sounds/SC_DoorOpen.SC_DoorOpen" (`self.K2_GetActorLocation`) (struct) 1.0 1.0 0.0 null null null null)))

(event `self.OpenDoor_Box_Small.OnComponentEndOverlap`
  (params (OverlappedComponent :type "PrimitiveComponent Object Reference") (OtherActor :type "Actor Object Reference") (OtherComp :type "PrimitiveComponent Object Reference") (OtherBodyIndex :type Integer))
  (if (== OtherActor (`GameplayStatics.GetPlayerCharacter` 0))
    (set `self.WantsOpen ` false)
    (`GameplayStatics.PlaySoundAtLocation` "/Game/Sounds/SC_DoorOpen.SC_DoorOpen" (`self.K2_GetActorLocation`) (struct) 1.0 1.0 0.0 null null null null)))

(event `self.ReceiveTick`
  (params (DeltaSeconds :type "Float (single-precision)"))
  (`SceneComponent.K2_SetRelativeLocation` (`self.SM_DoorPanel`) (`KismetMathLibrary.VInterpTo` (`SceneComponent.RelativeLocation` (`self.SM_DoorPanel`)) (`KismetMathLibrary.SelectVector` (`self.OpenLoc`) (`self.ClosedLoc`) (`self.WantsOpen `)) DeltaSeconds (`self.OpenSpeed`)) false false))

(fn `UserConstructionScript`)