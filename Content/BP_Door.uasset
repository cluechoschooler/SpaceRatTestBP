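; Sliding double door that also moves the player from the cargo hold to the crew quarters level.
; A trigger box plays a timeline that lerps the two door meshes apart when a Player-tagged component enters, and reverses it on exit.
; A second box shows a loading screen, then calls both stream-load and open-level on Lvl_CrewQuarters, followed by a stream-unload of Lvl_Cargohold, with level names hardcoded.
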(event `self.LoadNextLevel_Box.OnComponentBeginOverlap`
  (params (OverlappedComponent :type "PrimitiveComponent Object Reference") (OtherActor :type "Actor Object Reference") (OtherComp :type "PrimitiveComponent Object Reference") (OtherBodyIndex :type Integer) (bFromSweep :type Boolean) (SweepResult :type "HitResult Structure (by ref)"))
  (if (`ActorComponent.ComponentHasTag` OtherComp "Player")
    (bind _returnvalue (`|CreateWidget` "/Game/Levels/LoadingScreen.LoadingScreen_C"))
    (`UserWidget.AddToViewport` _returnvalue 0)
    (`GameplayStatics.LoadStreamLevel` "Lvl_CrewQuarters" true)
    (`GameplayStatics.OpenLevel` "Lvl_CrewQuarters")
    (`GameplayStatics.UnloadStreamLevel` "Lvl_Cargohold")))

(event `self.OpenDoor_Box.OnComponentBeginOverlap`
  (params (OverlappedComponent :type "PrimitiveComponent Object Reference") (OtherActor :type "Actor Object Reference") (OtherComp :type "PrimitiveComponent Object Reference") (OtherBodyIndex :type Integer) (bFromSweep :type Boolean) (SweepResult :type "HitResult Structure (by ref)"))
  (if (`ActorComponent.ComponentHasTag` OtherComp "Player")
    (bind (_direction _opendoortrack) (`Timeline|OpenDoorTL` :!label _label)
      (:`Update`
        (`SceneComponent.K2_SetRelativeLocation` (`self.SK_Door_left`) (`KismetMathLibrary.VLerp` (19.25 0.0 2.0) (19.25 120.0 2.0) _opendoortrack) false false)
        (`SceneComponent.K2_SetRelativeLocation` (`self.SK_Door_right`) (`KismetMathLibrary.VLerp` (17.514082 0.0 0.0) (17.514082 -110.0 0.0) _opendoortrack) false false)))))

(event `self.OpenDoor_Box.OnComponentEndOverlap`
  (params (OverlappedComponent :type "PrimitiveComponent Object Reference") (OtherActor :type "Actor Object Reference") (OtherComp :type "PrimitiveComponent Object Reference") (OtherBodyIndex :type Integer))
  (if (`ActorComponent.ComponentHasTag` OtherComp "Player")
    (goto _label :!via `Reverse`)))

(fn `UserConstructionScript`)