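; BP_Door_Clear is a double sliding door that opens while the player character is inside its trigger box.
; BeginPlay caches each panel's closed position and derives open positions offset in opposite Y directions.
; Box overlaps toggle a want-open flag and play the same sound at world origin for opening and closing.
; Tick uses VInterpTo to ease both panels toward the position that flag selects.
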(event `self.ReceiveBeginPlay`
  (`|ExecutionSequence`
    (:`then_0`
      (set `self.ClosedLoc_A` (`SceneComponent.RelativeLocation` (`self.SK_Door_left`))))
    (:`then_1`
      (set `self.ClosedLoc_B` (`SceneComponent.RelativeLocation` (`self.SK_Door_right`))))
    (:`then_2`
      (set `self.OpenLoc_A` (+ (`self.ClosedLoc_A`) (`KismetMathLibrary.MakeVector` 0.0 (`self.OpenDistance`)))))
    (:`then_3`
      (set `self.OpenLoc_B` (+ (`self.ClosedLoc_B`) (`KismetMathLibrary.MakeVector` 0.0 (* (`self.OpenDistance`) -1.0)))))))

(event `self.OpenDoor_Box.OnComponentBeginOverlap`
  (params (OverlappedComponent :type "PrimitiveComponent Object Reference") (OtherActor :type "Actor Object Reference") (OtherComp :type "PrimitiveComponent Object Reference") (OtherBodyIndex :type Integer) (bFromSweep :type Boolean) (SweepResult :type "HitResult Structure (by ref)"))
  (if (== OtherActor (`GameplayStatics.GetPlayerCharacter` 0))
    (set `self.bWantsOpen` true)
    (`GameplayStatics.PlaySoundAtLocation` "/Game/Sounds/SC_DoorOpen.SC_DoorOpen" (0.0 0.0 0.0) (struct) 1.0 1.0 0.0 null null null null)))

(event `self.OpenDoor_Box.OnComponentEndOverlap`
  (params (OverlappedComponent :type "PrimitiveComponent Object Reference") (OtherActor :type "Actor Object Reference") (OtherComp :type "PrimitiveComponent Object Reference") (OtherBodyIndex :type Integer))
  (if (== OtherActor (`GameplayStatics.GetPlayerCharacter` 0))
    (set `self.bWantsOpen` false)
    (`GameplayStatics.PlaySoundAtLocation` "/Game/Sounds/SC_DoorOpen.SC_DoorOpen" (0.0 0.0 0.0) (struct) 1.0 1.0 0.0 null null null null)))

(event `self.ReceiveTick`
  (params (DeltaSeconds :type "Float (single-precision)"))
  (`SceneComponent.K2_SetRelativeLocation` (`self.SK_Door_left`) (`KismetMathLibrary.VInterpTo` (`SceneComponent.RelativeLocation` (`self.SK_Door_left`)) (`KismetMathLibrary.SelectVector` (`self.OpenLoc_A`) (`self.ClosedLoc_A`) (`self.bWantsOpen`)) DeltaSeconds (`self.OpenSpeed`)) false false)
  (`SceneComponent.K2_SetRelativeLocation` (`self.SK_Door_right`) (`KismetMathLibrary.VInterpTo` (`SceneComponent.RelativeLocation` (`self.SK_Door_right`)) (`KismetMathLibrary.SelectVector` (`self.OpenLoc_B`) (`self.ClosedLoc_B`) (`self.bWantsOpen`)) DeltaSeconds (`self.OpenSpeed`)) false false))

(fn `UserConstructionScript`)