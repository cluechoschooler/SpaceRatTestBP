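; BP_AlarmLightController is an alarm light controller that blinks a set of lights together.
; BeginPlay starts a looping timer at BlinkInterval to drive the blinking.
; ToggleAlarm flips IsOn and sets the intensity of every light in AlarmLights to either OnIntensity or zero.
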(event `self.ReceiveBeginPlay`
  (`KismetSystemLibrary.K2_SetTimerDelegate` (`|CreateDelegate` :!event `ToggleAlarm`) (`self.BlinkInterval`) true))

(event `ToggleAlarm`
  (set `self.bIsOn` (not (`self.bIsOn`)))
  (for _array_element (`self.AlarmLights`)
    (`LightComponent.SetIntensity` (`Light.LightComponent` _array_element) (`KismetMathLibrary.SelectFloat` (`self.OnIntensity`) 0.0 (`self.bIsOn`)))))

(fn `UserConstructionScript`)